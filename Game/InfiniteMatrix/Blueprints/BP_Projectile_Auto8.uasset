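; BP_Projectile_Auto8 is a projectile that destroys enemies and adds to the player's score.
; On overlapping an Enemy_Blueprint, it increments the BP_Player score, updates the score bar and destroys both actors.
; Overlapping a BP_Tunnel destroys only the projectile.
; Every tick it sets its ProjectileMovement velocity along the X axis, scaling the initial speed by the player's current speed.
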(event `self.ReceiveActorBeginOverlap`
  (params (OtherActor :type "Actor Object Reference"))
  (bind _asenemy_blueprint (cast `/Game/InfiniteMatrix/Blueprints/Enemy_Blueprint` OtherActor)
    (:`then`
      (bind _asbp_player (cast `/Game/InfiniteMatrix/Blueprints/BP_Player` (`GameplayStatics.GetPlayerPawn` 0)))
      (bind _output_get (set `/Game/InfiniteMatrix/Blueprints/BP_Player.Score` (+ (`/Game/InfiniteMatrix/Blueprints/BP_Player.Score` _asbp_player) 1.0) _asbp_player))
      (`/Game/InfiniteMatrix/UI/WB_Score.Update Score` (`/Game/InfiniteMatrix/Blueprints/BP_Player.ScoreBar` _asbp_player) _output_get)
      (`self.K2_DestroyActor` _asenemy_blueprint)
      (`self.K2_DestroyActor`))
    (:`CastFailed`
      (cast `/Game/InfiniteMatrix/Blueprints/BP_Tunnel` OtherActor)
      (`self.K2_DestroyActor`))))

(event `self.ReceiveTick`
  (params (DeltaSeconds :type "Float (single-precision)"))
  (bind _projectilemovement (`self.ProjectileMovement`))
  (bind _asbp_player (cast `/Game/InfiniteMatrix/Blueprints/BP_Player` (`GameplayStatics.GetPlayerPawn` 0)))
  (set `MovementComponent.Velocity` (`KismetMathLibrary.MakeVector` (* (+ (* (`/Game/InfiniteMatrix/Blueprints/BP_Player.CurrentSpeed` _asbp_player) 0.025) 1.0) (`ProjectileMovementComponent.InitialSpeed` _projectilemovement))) _projectilemovement))

(fn `UserConstructionScript`)