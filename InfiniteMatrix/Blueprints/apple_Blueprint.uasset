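; Apple health pickup that randomly decides on BeginPlay whether to exist, surviving one time in five.
; A surviving apple instantly moves by a random positive offset on each axis.
; Overlapping a BP_Player below full health adds clamped health, updates the HealthBar widget and destroys the apple.
; SpawnApple spawns a scaled-up apple at a given location, with its random-chance check left disconnected.
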(event `self.ReceiveBeginPlay`
  (if (!= (`KismetMathLibrary.RandomIntegerInRange` 1 5) 5)
    (`self.K2_DestroyActor`)
    (else
      (`KismetSystemLibrary.MoveComponentTo` null (+ (`self.K2_GetActorLocation`) (`KismetMathLibrary.MakeVector` (`KismetMathLibrary.Conv_IntToDouble` (`KismetMathLibrary.RandomIntegerInRange` 0 800)) (`KismetMathLibrary.Conv_IntToDouble` (`KismetMathLibrary.RandomIntegerInRange` 0 800)) (`KismetMathLibrary.Conv_IntToDouble` (`KismetMathLibrary.RandomIntegerInRange` 0 800)))) (struct) false false 0.0))))

(event `self.ReceiveActorBeginOverlap`
  (params (OtherActor :type "Actor Object Reference"))
  (bind _asbp_player (cast `/Game/InfiniteMatrix/Blueprints/BP_Player` OtherActor))
  (if (< (`/Game/InfiniteMatrix/Blueprints/BP_Player.CurrentHealth` _asbp_player) 100.0)
    (bind _output_get (set `/Game/InfiniteMatrix/Blueprints/BP_Player.CurrentHealth` (`KismetMathLibrary.FClamp` (+ (`/Game/InfiniteMatrix/Blueprints/BP_Player.CurrentHealth` _asbp_player) 15.0) 0.0 100.0) _asbp_player))
    (`/Game/InfiniteMatrix/UI/WB_Health.UpdateHealth` (`/Game/InfiniteMatrix/Blueprints/BP_Player.HealthBar` _asbp_player) _output_get 100.0)
    (`self.K2_DestroyActor`)))

(fn `SpawnApple`
  (params (SpawnLocation :type "Vector Structure"))
  (`|SpawnActorFromClass` "apple_Blueprint_C" (`KismetMathLibrary.MakeTransform` SpawnLocation (struct) (1.3 1.3 1.3)) "Undefined" "MultiplyWithRoot" null null))

(fn `UserConstructionScript`)