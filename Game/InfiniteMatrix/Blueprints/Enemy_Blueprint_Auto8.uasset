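; Enemy actor that damages BP_Player on contact.
; On overlap it subtracts fixed health from the player and refreshes the health bar, then either flags the player dead and shows the restart screen, or destroys itself.
; A SpawnApple function spawns an enlarged Apple_Blueprint at a given location, but nothing here calls it and its random-chance check is disconnected.
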(event `self.ReceiveBeginPlay`)

(event `self.ReceiveActorBeginOverlap`
  (params (OtherActor :type "Actor Object Reference"))
  (bind _asbp_player (cast `/Game/InfiniteMatrix/Blueprints/BP_Player` OtherActor))
  (bind _output_get (set `/Game/InfiniteMatrix/Blueprints/BP_Player.CurrentHealth` (- (`/Game/InfiniteMatrix/Blueprints/BP_Player.CurrentHealth` _asbp_player) 25.0) _asbp_player))
  (`/Game/InfiniteMatrix/UI/WB_Health.UpdateHealth` (`/Game/InfiniteMatrix/Blueprints/BP_Player.HealthBar` _asbp_player) _output_get 100.0)
  (if (<= _output_get 0.0)
    (set `/Game/InfiniteMatrix/Blueprints/BP_Player.IsDead` true _asbp_player)
    (`/Game/InfiniteMatrix/Blueprints/BP_Player.DisplayRestart` _asbp_player)
    (else
      (`self.K2_DestroyActor`))))

(fn `SpawnApple`
  (params (SpawnLocation :type "Vector Structure"))
  (`|SpawnActorFromClass` "/Game/InfiniteMatrix/Blueprints/apple_Blueprint.apple_Blueprint_C" (`KismetMathLibrary.MakeTransform` SpawnLocation (struct) (1.3 1.3 1.3)) "Undefined" "MultiplyWithRoot" null null))

(fn `UserConstructionScript`)